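; Player interaction component for BP_FirstPersonCharacter that lets the player pick up, use and drop one held item.
; A self-repeating delayed sphere trace from the camera tracks the BPI_Item actor in view and shows a pickup prompt.
; E attaches it to HandHoldPoint, left mouse uses it and Q detaches it, each notifying the item through messages.
; An older line-trace door check is disconnected, leaving the CanOpenDoor click branch as a leftover.
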(event `self.ReceiveBeginPlay`
  (bind _asbp_first_person_character (cast `/Game/FirstPerson/Blueprints/BP_FirstPersonCharacter` (`self.GetOwner`)))
  (set `self. Player` _asbp_first_person_character)
  (set `self.First Person Camera` (`/Game/FirstPerson/Blueprints/BP_FirstPersonCharacter.FirstPersonCamera` _asbp_first_person_character))
  (`self.Looking`))

(event `Key|LeftMouseButton`
  (params (Key :type "Key Structure"))
  (:`Pressed`
    (if (`self.CanOpenDoor`)
      (`KismetSystemLibrary.PrintString` "Destory door"))))

(event `Looking`
  (bind _first_person_camera (`self.First Person Camera`))
  (bind _returnvalue (`SceneComponent.K2_GetComponentLocation` _first_person_camera))
  (`KismetSystemLibrary.Delay` (`self.Interact Interval`))
  (bind (_outhit _returnvalue_2) (`KismetSystemLibrary.SphereTraceSingle` :`Start` _returnvalue :`End` (+ _returnvalue (* (`SceneComponent.GetForwardVector` _first_person_camera) (`self.Look Distance`))) :`Radius` 20.0 :`TraceChannel` "TraceTypeQuery1" :`DrawTime` 1.0))
  (if _returnvalue_2
    (bind (_bblockinghit _binitialoverlap _time _distance _location _impactpoint _normal _impactnormal _physmat _hitactor) (`GameplayStatics.BreakHitResult` _outhit))
    (if (`KismetSystemLibrary.DoesImplementInterface` _hitactor "/Game/Blueprints/BPI_Item.BPI_Item_C")
      (set `self.Last Touched Item` _hitactor) ; Keep track of what we touched
      (`KismetSystemLibrary.PrintText` (`|FormatText` "Pess E to pick up {name}." (`KismetSystemLibrary.GetDisplayName` _hitactor)) true true (struct :`G` 0.66 :`B` 1.0 :`A` 1.0) (`self.Interact Interval`))
      (else
        (set `self.Last Touched Item` null)))
    (else
      (set `self.Last Touched Item` null) ; If i see nothing reset last touched
    ))
  (`self.Looking`))

(event `Key|E`
  (params (Key :type "Key Structure"))
  (:`Pressed`
    (`self.Try to pick up`)))

(event `Try to pick up`
  (`self.Held Item`
    (:`then`
      (`KismetSystemLibrary.PrintText` "We're already hold something!"))
    (:`else`
      (bind _last_touched_item (`self.Last Touched Item`)
        (:`then`
          (message `/Game/Blueprints/BPI_Item.PickUp` _last_touched_item self)
          (`Actor.K2_AttachToComponent` _last_touched_item (`/Game/FirstPerson/Blueprints/BP_FirstPersonCharacter.HandHoldPoint` (`self. Player`)) "None" "SnapToTarget" "SnapToTarget" "KeepRelative" true)
          (set `self.Held Item` _last_touched_item)
          (set `self.Last Touched Item` null))
        (:`else`
          (`KismetSystemLibrary.PrintText` "We're not looking at anything."))))))

(event `Try to Use`
  (bind _held_item (`self.Held Item`)
    (:`then`
      (message `/Game/Blueprints/BPI_Item.Use` _held_item))
    (:`else`
      (`KismetSystemLibrary.PrintText` "We aren't holding anything."))))

(event `Key|LeftMouseButton`
  (params (Key :type "Key Structure"))
  (:`Pressed`
    (`self.Try to Use`)))

(event `Key|Q`
  (params (Key :type "Key Structure"))
  (:`Pressed`
    (`self.Try to Drop`)))

(event `Try to Drop`
  (bind _held_item (`self.Held Item`)
    (:`then`
      (`Actor.K2_DetachFromActor` _held_item "KeepRelative" "KeepRelative" "KeepRelative")
      (`Actor.K2_DetachFromActor` (`self.Held Item`) "KeepRelative" "KeepRelative" "KeepRelative")
      (message `/Game/Blueprints/BPI_Item.Drop` _held_item)
      (set `self.Held Item` null))
    (:`else`)))