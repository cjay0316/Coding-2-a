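; BP_BirdsEye is a trigger actor that briefly shows the player an alternate bird's-eye camera view.
; When BP_FirstPersonCharacter overlaps the Trigger, it disables input and cubic-blends the view target to BirdsEyeCamera.
; After the blend and a short hold, it starts blending back to the character and re-enables input shortly afterward, without waiting for that blend to complete.
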(event `self.Trigger.OnComponentBeginOverlap`
  (params (OverlappedComponent :type "PrimitiveComponent Object Reference") (OtherActor :type "Actor Object Reference") (OtherComp :type "PrimitiveComponent Object Reference") (OtherBodyIndex :type Integer) (bFromSweep :type Boolean) (SweepResult :type "HitResult Structure (by ref)"))
  (bind _returnvalue (`GameplayStatics.GetPlayerController` 0))
  (bind _returnvalue_2 (`GameplayStatics.GetPlayerController` 0))
  (bind _blend_time (`self.Blend Time`))
  (cast `/Game/FirstPerson/Blueprints/BP_FirstPersonCharacter` OtherActor)
  (`self.DisableInput` _returnvalue_2 _returnvalue_2)
  (`PlayerController.SetViewTargetWithBlend` (`GameplayStatics.GetPlayerController` 0) (`self.BirdsEyeCamera`) _blend_time "VTBlend_Cubic" 1.0 false)
  (`KismetSystemLibrary.Delay` _blend_time)
  (`KismetSystemLibrary.Delay` 1.0)
  (`PlayerController.SetViewTargetWithBlend` (`GameplayStatics.GetPlayerController` 0) OtherActor _blend_time "VTBlend_Cubic" 1.0 false)
  (`KismetSystemLibrary.Delay` 0.2)
  (`self.EnableInput` _returnvalue _returnvalue))

(fn `UserConstructionScript`)